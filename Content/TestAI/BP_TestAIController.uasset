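; AI controller that drives BP_TestAI or BP_AI_Background pawns through the BT_AI_Base behavior tree.
; On possess it caches the pawn and sorts tagged TargetPoint actors into two patrol lists, which GetNewPoint cycles into the blackboard by path index.
; AI Perception updates player visibility on the blackboard and records the player's location when sight is lost.
; Walk and Run events forward gait changes to the cached pawns.
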(event `Walk`
  (bind _backgroundai (`self.BackgroundAI`))
  (`/Game/TestAI/BP_TestAI.Walk` (`self.TestAI`))
  (if (`KismetSystemLibrary.IsValid` _backgroundai)
    (`/Game/TestAI/BP_AI_Background.Walk` _backgroundai)))

(event `Run`
  (bind _backgroundai (`self.BackgroundAI`))
  (`/Game/TestAI/BP_TestAI.Run` (`self.TestAI`))
  (if (`KismetSystemLibrary.IsValid` _backgroundai)
    (`/Game/TestAI/BP_AI_Background.Run` _backgroundai)))

(event `self.OnPossess`
  (params (PossessedPawn :type "Pawn Object Reference"))
  (bind _asbp_test_ai (cast `/Game/TestAI/BP_TestAI` PossessedPawn)
    (:`then`
      (set `self.TestAI` _asbp_test_ai))
    (:`CastFailed`
      (bind _asbp_ai_background (cast `/Game/TestAI/BP_AI_Background` PossessedPawn))
      (set `self.BackgroundAI` _asbp_ai_background)))
  (`self.RunBehaviorTree` "/Game/TestAI/BT_AI_Base.BT_AI_Base")
  (bind _outactors (`GameplayStatics.GetAllActorsOfClass` "/Script/Engine.TargetPoint"))
  (for _array_element _outactors
    (if (`self.ActorHasTag` _array_element "TargetPoint")
      (`KismetArrayLibrary.Array_Add` (`self.TargetPoints`) _array_element)
      (elif (`self.ActorHasTag` _array_element "TargetPoint2")
        (`KismetArrayLibrary.Array_Add` (`self.TargetPoints2`) _array_element))))
  (set `self.TotalTargets` (`KismetArrayLibrary.Array_Length` (`self.TargetPoints`))))

(event `self.AIPerception.OnTargetPerceptionUpdated`
  (params (Actor :type "Actor Object Reference") (Stimulus :type "AIStimulus Structure"))
  (bind (_age _expirationage _strength _stimuluslocation _receiverlocation _tag _bsuccessfullysensed) (break `AIStimulus` Stimulus))
  (bind _returnvalue (`AIBlueprintHelperLibrary.GetBlackboard` null))
  (cast `/Game/BP_PlayerCharacter` Actor)
  (`BlackboardComponent.SetValueAsBool` _returnvalue "CanSeePlayer" _bsuccessfullysensed)
  (if (not _bsuccessfullysensed)
    (`BlackboardComponent.SetValueAsVector` _returnvalue "PlayerLoc" (`self.K2_GetActorLocation` (`GameplayStatics.GetPlayerCharacter` 0)))
    (`BlackboardComponent.SetValueAsBool` _returnvalue "RecentlySeen" true)))

(event `GetNewPoint`
  (params (Path :type Integer))
  (switch `int` Path
    (:`0`
      (if (not (`KismetSystemLibrary.IsValid` (`|GetArrayItem` (`self.TargetPoints`) (`self.CurTargetPoint`))))
        (set `self.CurTargetPoint` 0))
      (`BlackboardComponent.SetValueAsObject` (`AIBlueprintHelperLibrary.GetBlackboard` null) "TargetPointKey" (`|GetArrayItem` (`self.TargetPoints`) (`self.CurTargetPoint`)))
      (bind _result (`/Engine/EditorBlueprintResources/StandardMacros.IncrementInt` (`self.CurTargetPoint`))
        (:`  `
          (set `self.CurTargetPoint` _result))))
    (:`1`
      (if (not (`KismetSystemLibrary.IsValid` (`|GetArrayItem` (`self.TargetPoints2`) (`self.CurTargetPoint2`))))
        (set `self.CurTargetPoint2` 0))
      (`BlackboardComponent.SetValueAsObject` (`AIBlueprintHelperLibrary.GetBlackboard` null) "TargetPointKey" (`|GetArrayItem` (`self.TargetPoints2`) (`self.CurTargetPoint2`)))
      (bind _result_2 (`/Engine/EditorBlueprintResources/StandardMacros.IncrementInt` (`self.CurTargetPoint2`))
        (:`  `
          (set `self.CurTargetPoint2` _result_2))))))

(fn `UserConstructionScript`)