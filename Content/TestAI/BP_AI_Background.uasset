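; Test AI character that switches between walking and alerted running, and reports to MyGameMode when it overlaps the player while alerted.
; Walk and Run events set speed, sphere material and the PlayerDetected flag.
; ConeCreation converts EQS result points into a triangle fan and builds a procedural vision cone mesh from it.
; The EQS_VisionCone query that would feed it is disconnected, so nothing here triggers the cone.
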(event `self.ReceiveTick`
  (params (DeltaSeconds :type "Float (single-precision)")))

(event `ConeCreation`
  (params (QueryInstance :type "EnvQueryInstanceBlueprintWrapper Object Reference") (QueryStatus :type "EEnvQueryStatus Enum" :default "Processing"))
  (bind _output_get (set `self.SightPoints` (`EnvQueryInstanceBlueprintWrapper.GetResultsAsLocations` QueryInstance)))
  (bind (_vertices _triangles) (`self.ConvertSightPoints` _output_get))
  (`self.CreatingCone` _vertices _triangles))

(event `self.ReceiveBeginPlay`
  (`KismetArrayLibrary.Array_Resize` (`self.Vertices`) 51)
  (set `self.REFDefaultMaterial` (`PrimitiveComponent.GetMaterial` (`self.Sphere`) 0))
  (set `self.REFPlayer` (`GameplayStatics.GetPlayerCharacter` 0))
  (set `self.REFGameMode` (`GameplayStatics.GetGameMode`))
  (bind _asbp_test_aicontroller (cast `/Game/TestAI/BP_TestAIController` (`self.GetController`)))
  (set `self.REFAIController` _asbp_test_aicontroller))

(event `Walk`
  (set `CharacterMovementComponent.MaxWalkSpeed` 200.0 (`self.CharacterMovement`))
  (`PrimitiveComponent.SetMaterial` (`self.Sphere`) 0 (`self.REFDefaultMaterial`))
  (set `self.PlayerDetected` false))

(event `Run`
  (set `CharacterMovementComponent.MaxWalkSpeed` 325.0 (`self.CharacterMovement`))
  (`PrimitiveComponent.SetMaterial` (`self.Sphere`) 0 "/Game/M_Alert.M_Alert")
  (set `self.PlayerDetected` true))

(event `self.ReceiveActorBeginOverlap`
  (params (OtherActor :type "Actor Object Reference"))
  (cast `/Game/Blueprints/BP_PlayerCharacter` OtherActor)
  (bind _asmy_game_mode (cast `/Game/Blueprints/MyGameMode` (`GameplayStatics.GetGameMode`)))
  (if (`self.PlayerDetected`)
    (`/Game/Blueprints/MyGameMode.Detected` _asmy_game_mode)))

(fn `ConvertSightPoints`
  (params (SightPoints :type "Array of Vector Structure"))
  (returns (Vertices :type "Array of Vector Structure") (Triangles :type "Array of Integer"))
  (bind _returnvalue (* 3 (`KismetArrayLibrary.Array_Length` (`self.Vertices`))))
  (`KismetArrayLibrary.Array_Set` (`self.Vertices`))
  (for (_array_element _array_index) SightPoints
    (`KismetArrayLibrary.Array_Set` (`self.Vertices`) _array_index (`KismetMathLibrary.MakeVector` (- (.x _array_element) (.x (`self.K2_GetActorLocation`))) (- (.y _array_element) (.y (`self.K2_GetActorLocation`))) -50.0)))
  (`KismetArrayLibrary.Array_Resize` (`self.Triangles`) _returnvalue)
  (for _index (range (+ _returnvalue 1))
    (bind _returnvalue_2 (* _index 3))
    (`KismetArrayLibrary.Array_Set` (`self.Triangles`) _returnvalue_2)
    (bind _returnvalue_3 (+ _returnvalue_2 1))
    (bind _returnvalue_4 (+ _index 1))
    (`KismetArrayLibrary.Array_Set` (`self.Triangles`) _returnvalue_3 _returnvalue_4)
    (`KismetArrayLibrary.Array_Set` (`self.Triangles`) (+ _returnvalue_3 1) (+ _returnvalue_4 1)))
  (return (`self.Vertices`) (`self.Triangles`)))

(fn `CreatingCone`
  (params (Vertices :type "Array of Vector Structure") (Triangles :type "Array of Integer"))
  (bind _visioncone (`self.VisionCone`))
  (`ProceduralMeshComponent.CreateMeshSection_LinearColor` :`self` _visioncone :`Vertices` Vertices :`Triangles` Triangles)
  (`PrimitiveComponent.SetMaterial` _visioncone 0 "/Game/M_Alert.M_Alert")
  (`SceneComponent.K2_SetWorldRotation` :`self` _visioncone))

(fn `UserConstructionScript`)