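; Base AI character that patrols target points and reports to the game mode when it first sees the player.
; On BeginPlay it gathers all TargetPoints and runs Wait or Patrol from AIState, looping through targets with AIMoveTo and pauses.
; Failed moves or overlaps with the player or a block stop movement, step the target index back and re-run the behavior.
; A sighting, gated by DoOnce, swaps the sphere to an alert material, waits, then calls Detected.
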(event `self.ReceiveBeginPlay`
  (set `self.REFOriginalMaterial` (`PrimitiveComponent.GetMaterial` (`self.Sphere`) 0))
  (bind _outactors (`GameplayStatics.GetAllActorsOfClass` "/Script/Engine.TargetPoint"))
  (set `self.Targets` _outactors)
  (`self.Behavior`))

(event `Behavior`
  (switch `/Game/E_AIState` (`self.AIState`)
    (:`NewEnumerator0`
      (`self.Wait`))
    (:`NewEnumerator1`
      (`self.Patrol`))))

(event `Patrol`
  (if (not (`KismetSystemLibrary.IsValid` (`|GetArrayItem` (`self.Targets`) (`self.CurTarget`))))
    (set `self.CurTarget` 0))
  (`|AIMoveTo` self (0.0 0.0 0.0) (`|GetArrayItem` (`self.Targets`) (`self.CurTarget`)) 5.0 true
    (:`OnSuccess`
      (set `self.CurTarget` (+ (`self.CurTarget`) 1))
      (`KismetSystemLibrary.Delay` 2.0)
      (`self.Patrol`))
    (:`OnFail`
      (`self.Wait`))))

(event `Wait`
  (`NavMovementComponent.StopActiveMovement` (`self.CharacterMovement`))
  (set `self.CurTarget` (- (`self.CurTarget`) 1))
  (`KismetSystemLibrary.Delay` 2.0)
  (`self.Behavior`))

(event `self.ReceiveActorBeginOverlap`
  (params (OtherActor :type "Actor Object Reference"))
  (cast `/Game/BP_PlayerCharacter` OtherActor
    (:`then`
      _)
    (:`CastFailed`
      (cast `/Game/BP_Block` OtherActor)))
  (`self.Wait`))

(event `self.PawnSensing.OnSeePawn`
  (params (Pawn :type "Pawn Object Reference"))
  (`/Engine/EditorBlueprintResources/StandardMacros.DoOnce` false
    (:`Completed`
      (cast `/Game/BP_PlayerCharacter` Pawn)
      (`PrimitiveComponent.SetMaterial` (`self.Sphere`) 0 "/Game/M_Alert.M_Alert")
      (`self.Wait`)
      (`KismetSystemLibrary.Delay` 1.0)
      (bind _asmy_game_mode (cast `/Game/MyGameMode` (`GameplayStatics.GetGameMode`)))
      (`/Game/MyGameMode.Detected` _asmy_game_mode))))

(fn `UserConstructionScript`)