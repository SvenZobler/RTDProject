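; BP_NewBlock is a block actor whose static mesh simulates physics only in response to the player's proximity.
; Two trigger volumes, XBox and YBox, enable simulation when a BP_NewPlayer begins overlapping and disable it when the overlap ends.
; The boxes share no state, so leaving either one turns physics off even if the player is still inside the other.
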(event `self.YBox.OnComponentBeginOverlap`
  (params (OverlappedComponent :type "PrimitiveComponent Object Reference") (OtherActor :type "Actor Object Reference") (OtherComp :type "PrimitiveComponent Object Reference") (OtherBodyIndex :type Integer) (bFromSweep :type Boolean) (SweepResult :type "HitResult Structure (by ref)"))
  (cast `/Game/Blueprints/BP_NewPlayer` OtherActor)
  (`PrimitiveComponent.SetSimulatePhysics` (`self.StaticMesh`) true))

(event `self.YBox.OnComponentEndOverlap`
  (params (OverlappedComponent :type "PrimitiveComponent Object Reference") (OtherActor :type "Actor Object Reference") (OtherComp :type "PrimitiveComponent Object Reference") (OtherBodyIndex :type Integer))
  (cast `/Game/Blueprints/BP_NewPlayer` OtherActor)
  (`PrimitiveComponent.SetSimulatePhysics` (`self.StaticMesh`) false))

(event `self.XBox.OnComponentBeginOverlap`
  (params (OverlappedComponent :type "PrimitiveComponent Object Reference") (OtherActor :type "Actor Object Reference") (OtherComp :type "PrimitiveComponent Object Reference") (OtherBodyIndex :type Integer) (bFromSweep :type Boolean) (SweepResult :type "HitResult Structure (by ref)"))
  (cast `/Game/Blueprints/BP_NewPlayer` OtherActor)
  (`PrimitiveComponent.SetSimulatePhysics` (`self.StaticMesh`) true))

(event `self.XBox.OnComponentEndOverlap`
  (params (OverlappedComponent :type "PrimitiveComponent Object Reference") (OtherActor :type "Actor Object Reference") (OtherComp :type "PrimitiveComponent Object Reference") (OtherBodyIndex :type Integer))
  (cast `/Game/Blueprints/BP_NewPlayer` OtherActor)
  (`PrimitiveComponent.SetSimulatePhysics` (`self.StaticMesh`) false))

(fn `UserConstructionScript`)