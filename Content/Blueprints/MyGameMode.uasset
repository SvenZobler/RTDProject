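; Game mode that handles the end of a level, either by completion or by the player being detected.
; BeginPlay pre-creates the level-win, game-win and detected widgets; LevelComplete picks a win screen by comparing current and max level from MyGameInstance.
; Detected runs once, then joins LevelComplete's tail, which disables input, shows the cursor and sets LevelWon even on detection.
; Also holds two loop macros for stepped or delayed iteration, unused in its event graph.
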(event `self.ReceiveBeginPlay`
  (bind _output_get (set `self.REFPlayerController` (`GameplayStatics.GetPlayerController` 0)))
  (bind _returnvalue (`|CreateWidget` "/Game/UI/W_LevelWin.W_LevelWin_C" _output_get))
  (set `self.REFLevelWin` _returnvalue)
  (bind _returnvalue_2 (`|CreateWidget` "/Game/UI/W_DetectedText.W_DetectedText_C" (`self.REFPlayerController`)))
  (set `self.REFDetectedWidget` _returnvalue_2)
  (bind _returnvalue_3 (`|CreateWidget` "/Game/UI/W_GameWin.W_GameWin_C" (`self.REFPlayerController`)))
  (set `self.REFGameWin` _returnvalue_3)
  (set `self.LevelWon` false))

(event `LevelComplete`
  (bind _refplayercontroller (`self.REFPlayerController`))
  (bind _asmy_game_instance (cast `/Game/Blueprints/MyGameInstance` (`GameplayStatics.GetGameInstance`)))
  (if (>= (`/Game/Blueprints/MyGameInstance.curLevel` _asmy_game_instance) (`/Game/Blueprints/MyGameInstance.maxLevel` _asmy_game_instance))
    (`UserWidget.AddToViewport` (`self.REFGameWin`) 0)
    (else
      (`UserWidget.AddToViewport` (`self.REFLevelWin`) 0)))
  (`self.DisableInput` (`GameplayStatics.GetPlayerCharacter` 0) _refplayercontroller :!label _label)
  (set `PlayerController.bShowMouseCursor` true _refplayercontroller)
  (set `self.LevelWon` true))

(event `Detected`
  (`/Engine/EditorBlueprintResources/StandardMacros.DoOnce` false
    (:`Completed`
      (`UserWidget.AddToViewport` (`self.REFDetectedWidget`) 0)
      (goto _label))))

(fn `UserConstructionScript`)