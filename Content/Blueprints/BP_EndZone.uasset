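; BP_EndZone is an end-of-level trigger that completes the level when the player reaches it.
; On actor overlap it checks for a BP_NewPlayer, then calls LevelComplete on MyGameMode.
; Unconnected leftover nodes reference BP_Block and a BP_PlayerCharacter Detach call, but they never run.
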(event `self.ReceiveBeginPlay`)

(event `self.ReceiveActorBeginOverlap`
  (params (OtherActor :type "Actor Object Reference"))
  (cast `/Game/Blueprints/BP_NewPlayer` OtherActor)
  (bind _asmy_game_mode (cast `/Game/Blueprints/MyGameMode` (`GameplayStatics.GetGameMode`)))
  (`/Game/Blueprints/MyGameMode.LevelComplete` _asmy_game_mode))

(fn `UserConstructionScript`)