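; Player character that moves along fixed world axes and can pick up, carry and release BP_Block actors.
; Overlap events track the current block and whether Interact can act on it.
; Interact toggles attaching the block to the character, disabling the block's cube collision while held and restoring it on detach.
; CubeHeld and CubeReleased switch max walk speed between carrying and default values.
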(event `InputAxis|Forward`
  (params (AxisValue :type "Float (single-precision)"))
  ;[1 1 1] Basic Movement
  (`self.AddMovementInput` (1.0 0.0 0.0) AxisValue))

(event `InputAxis|Left`
  (params (AxisValue :type "Float (single-precision)"))
  ;[1 1 1] Basic Movement
  (`self.AddMovementInput` (0.0 -1.0 0.0) AxisValue))

(event `InputAxis|Backward`
  (params (AxisValue :type "Float (single-precision)"))
  ;[1 1 1] Basic Movement
  (`self.AddMovementInput` (-1.0 0.0 0.0) AxisValue))

(event `InputAxis|Right`
  (params (AxisValue :type "Float (single-precision)"))
  ;[1 1 1] Basic Movement
  (`self.AddMovementInput` (0.0 1.0 0.0) AxisValue))

(event `self.ReceiveActorBeginOverlap`
  (params (OtherActor :type "Actor Object Reference"))
  ;[1 1 1] Block Logic
  (bind _asbp_block (cast `/Game/Blueprints/BP_Block` OtherActor))
  (set `self.curBlock` _asbp_block)
  (if (`self.IsOverlappingActor` _asbp_block)
    (set `self.IsOverlapping` true)))

(event `self.ReceiveActorEndOverlap`
  (params (OtherActor :type "Actor Object Reference"))
  ;[1 1 1] Block Logic
  (bind _asbp_block (cast `/Game/Blueprints/BP_Block` OtherActor))
  (if (not (`self.IsOverlappingActor` _asbp_block))
    (set `self.IsOverlapping` false)))

(event `InputAction|Interact`
  (params (Key :type "Key Structure"))
  (bind _curblock (`self.curBlock`))
  (bind _cube (`/Game/Blueprints/BP_Block.Cube` _curblock))
  ;[1 1 1] Block Logic
  (:`Pressed`
    (if (`self.IsOverlapping`)
      (if (`self.IsAttached`)
        (`self.Detach` _curblock _cube)
        (else
          (`self.K2_AttachToActor` _curblock self "None" "KeepWorld" "KeepWorld" "KeepWorld" true)
          (set `self.IsAttached` true)
          (`self.CubeHeld`)
          (bind _output_get (set `self.CurBlockCollision` _cube))
          (`PrimitiveComponent.SetCollisionEnabled` _output_get "NoCollision"))))))

(fn `CubeHeld`
  (set `CharacterMovementComponent.MaxWalkSpeed` (`self.BlockWalkSpeed`) (`self.CharacterMovement`)))

(fn `CubeReleased`
  (set `CharacterMovementComponent.MaxWalkSpeed` (`self.DefaultWalkSpeed`) (`self.CharacterMovement`)))

(fn `Detach`
  (params (CubeRef :type "Actor Object Reference") (CubeCollision :type "PrimitiveComponent Object Reference"))
  (`self.K2_DetachFromActor` CubeRef "KeepWorld" "KeepWorld" "KeepWorld")
  (set `self.IsAttached` false)
  (`self.CubeReleased`)
  (`PrimitiveComponent.SetCollisionEnabled` (`self.CurBlockCollision`) "QueryAndPhysics"))

(fn `UserConstructionScript`)