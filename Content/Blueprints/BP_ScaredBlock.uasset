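; BP_ScaredBlock is a moving block actor with partially built logic for attaching to and detaching from the player.
; On BeginPlay, a timeline repeatedly nudges it from its current location along a mostly-X offset, so movement accumulates.
; Detach calls DetachFromActor on the overlapping player character rather than on the block.
; Attach is empty, the toggle that would attach the block to the player is unwired, and its helper functions are stubs.
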(event `self.ReceiveBeginPlay`
  (bind _returnvalue (`self.K2_GetActorLocation`))
  (bind (_direction _newtrack_0) (`Timeline|Timeline_0` :!via `PlayFromStart`)
    (:`Update`
      (`self.K2_SetActorLocation` (`KismetMathLibrary.VLerp` _returnvalue (+ _returnvalue (3.5 0.5 0.0)) _newtrack_0)))))

(event `self.ReceiveActorBeginOverlap`
  (params (OtherActor :type "Actor Object Reference")))

(event `Attach`)

(event `Detach`
  (bind _asbp_player_character (cast `/Game/Blueprints/BP_PlayerCharacter` (`GameplayStatics.GetPlayerCharacter` 0)))
  (if (`self.IsOverlappingActor` _asbp_player_character)
    (`self.K2_DetachFromActor` _asbp_player_character "KeepRelative" "KeepRelative" "KeepRelative")
    (set `self.IsAttached` false)))

(fn `AttachToPlayer`)

(fn `Countdown`)

(fn `GetLoc`
  (params (NewParam1 :type "Vector Structure"))
  (returns (NewParam :type "Vector Structure"))
  (return (0.0 0.0 0.0)))

(fn `UserConstructionScript`)