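; BP_Block is a block actor with unfinished logic for attaching to and detaching from the player character.
; Its Detach event checks for overlap with the player, then calls DetachFromActor on the player rather than the block and clears IsAttached.
; An unconnected toggle branch would attach the block to an overlapping player or reuse the detach path.
; The Attach event, overlap event, AttachToPlayer and Countdown are empty.
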(event `self.ReceiveActorBeginOverlap`
  (params (OtherActor :type "Actor Object Reference")))

(event `Attach`)

(event `Detach`
  (bind _asbp_player_character (cast `/Game/BP_PlayerCharacter` (`GameplayStatics.GetPlayerCharacter` 0)))
  (if (`self.IsOverlappingActor` _asbp_player_character)
    (`self.K2_DetachFromActor` _asbp_player_character "KeepRelative" "KeepRelative" "KeepRelative")
    (set `self.IsAttached` false)))

(fn `AttachToPlayer`)

(fn `Countdown`)

(fn `UserConstructionScript`)